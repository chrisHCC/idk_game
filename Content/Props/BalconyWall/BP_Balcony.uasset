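; Spline-driven balcony wall prop that builds its geometry in the construction script, with no active runtime logic.
; It adds one spline mesh component per segment between spline points, attached to the root and bent to the local positions and tangents at both ends.
; First, last and middle segments each use a separate Add Spline Mesh node, allowing distinct templates for end and middle pieces.
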(fn `UserConstructionScript`
  (bind _spline (`self.Spline`))
  (bind _returnvalue (`SplineComponent.GetNumberOfSplinePoints` _spline))
  (for _index (range (+ (- _returnvalue 2) 1))
    (if (== _index 0)
      (bind _returnvalue_2 (`AddComponent|NODE_AddSplineMeshComponent-2`))
      (`SceneComponent.K2_AttachToComponent` _returnvalue_2 (`self.DefaultSceneRoot`) "None" "KeepRelative" "KeepRelative" "KeepRelative" true)
      (bind (_location _tangent) (`SplineComponent.GetLocationAndTangentAtSplinePoint` _spline _index "Local"))
      (bind (_location_2 _tangent_2) (`SplineComponent.GetLocationAndTangentAtSplinePoint` _spline (+ _index 1) "Local"))
      (`SplineMeshComponent.SetStartAndEnd` _returnvalue_2 _location _tangent _location_2 _tangent_2 true)
      (elif (== (- _returnvalue 2) _index)
        (bind _returnvalue_3 (`AddComponent|NODE_AddSplineMeshComponent-4`))
        (`SceneComponent.K2_AttachToComponent` _returnvalue_3 (`self.DefaultSceneRoot`) "None" "KeepRelative" "KeepRelative" "KeepRelative" true)
        (bind (_location_3 _tangent_3) (`SplineComponent.GetLocationAndTangentAtSplinePoint` _spline _index "Local"))
        (bind (_location_4 _tangent_4) (`SplineComponent.GetLocationAndTangentAtSplinePoint` _spline (+ _index 1) "Local"))
        (`SplineMeshComponent.SetStartAndEnd` _returnvalue_3 _location_3 _tangent_3 _location_4 _tangent_4 true)
        (else
          (bind _returnvalue_4 (`AddComponent|NODE_AddSplineMeshComponent-0`))
          (`SceneComponent.K2_AttachToComponent` _returnvalue_4 (`self.DefaultSceneRoot`) "None" "KeepRelative" "KeepRelative" "KeepRelative" true)
          (bind (_location_5 _tangent_5) (`SplineComponent.GetLocationAndTangentAtSplinePoint` _spline _index "Local"))
          (bind (_location_6 _tangent_6) (`SplineComponent.GetLocationAndTangentAtSplinePoint` _spline (+ _index 1) "Local"))
          (`SplineMeshComponent.SetStartAndEnd` _returnvalue_4 _location_5 _tangent_5 _location_6 _tangent_6 true))))))