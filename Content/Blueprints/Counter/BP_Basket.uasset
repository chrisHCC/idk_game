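; BP_Basket is a counter that tallies overlaps ending on its Box and switches on selected actors once a threshold is reached.
; Each end overlap raises Total by Add1 and shows the new count on a TextRender, with no filter on the overlapping actor.
; While Total is at or above SetMax, each such event sends ToggleStateMessage(true) to every actor in SelectAffectedActors, so it repeats on later overlaps.
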(event `self.Box.OnComponentEndOverlap`
  (params (OverlappedComponent :type "PrimitiveComponent Object Reference") (OtherActor :type "Actor Object Reference") (OtherComp :type "PrimitiveComponent Object Reference") (OtherBodyIndex :type Integer))
  (bind _returnvalue (+ (`self.total`) (`self.add1`)))
  (`TextRenderComponent.K2_SetText` (`self.TextRender`) (`KismetTextLibrary.Conv_IntToText` _returnvalue))
  (set `self.total` _returnvalue)
  (if (>= (`self.total`) (`self.Set Max`))
    (for _array_element (`self.Select Affected Actors`)
      (message `/Game/Blueprints/Player/LaserState.ToggleState` _array_element true))))

(fn `UserConstructionScript`)