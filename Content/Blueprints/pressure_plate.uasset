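; Pressure plate actor that shows a Good or Bad verdict on a text render, based on a pickup cube's weight.
; When its box begins an overlap, it fetches all BP_PickupCube actors and compares the first one's Weight to an exact target value.
; The check ignores which actor overlapped the plate.
; An Mcpawn lookup also runs, but its result and held-object reference do not affect the outcome.
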(event `self.ReceiveBeginPlay`)

(event `self.Box.OnComponentBeginOverlap`
  (params (OverlappedComponent :type "PrimitiveComponent Object Reference") (OtherActor :type "Actor Object Reference") (OtherComp :type "PrimitiveComponent Object Reference") (OtherBodyIndex :type Integer) (bFromSweep :type Boolean) (SweepResult :type "HitResult Structure (by ref)"))
  (bind _textrender (`self.TextRender`))
  (bind _outactors (`GameplayStatics.GetAllActorsOfClass` "/Game/Blueprints/Player/mcpawn.mcpawn_C"))
  (bind _outactors_2 (`GameplayStatics.GetAllActorsOfClass` "/Game/Blueprints/BP_PickupCube.BP_PickupCube_C"))
  (if (== (`/Game/Blueprints/BP_PickupCube.Weight` (`|GetArrayItem` _outactors_2)) 120.0)
    (`TextRenderComponent.K2_SetText` _textrender (`self.good`))
    (else
      (`TextRenderComponent.K2_SetText` _textrender (`self.bad`)))))

(fn `UserConstructionScript`)