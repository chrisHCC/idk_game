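; Static laser refractor that, when toggled, emits a beam along its arrow and passes the laser on to whatever it hits.
; CastLight line-traces on Visibility and sets the particle beam's endpoints to the origin and the impact point or max range.
; The hit face's material identifies receivers and other refractors, which get a toggle message so beams can chain.
; After a one-second delay the beam hides unless LaserStaysOn is set.
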(event `/Game/Blueprints/Player/LaserState.ToggleState`
  (params (`On/Off` :type Boolean))
  (bind _particlesystem (`self.ParticleSystem`))
  (bind _arrow (`self.Arrow`))
  (set `self.isOn` `On/Off`)
  (`SceneComponent.SetVisibility` (`self.ParticleSystem`) true false)
  (`self.CastLight` self (`SceneComponent.K2_GetComponentLocation` _arrow) (`SceneComponent.GetForwardVector` _arrow) (`self.Max Distance Laser`))
  (`KismetSystemLibrary.Delay` 1.0)
  (if (`self.laser stays on`)
    (`SceneComponent.SetVisibility` _particlesystem true false)
    (set `self.isOn` true)
    (else
      (`SceneComponent.SetVisibility` _particlesystem false false)
      (set `self.isOn` false))))

(event `self.ReceiveTick`
  (params (DeltaSeconds :type "Float (single-precision)"))
  (if (`self.isOn`)
    _))

(fn `CastLight`
  (params (Origin :type "Vector Structure") (Direction :type "Vector Structure") (Distance :type "Float (double-precision)"))
  (locals (L_Origin :type "Vector Structure") (L_Direction :type "Vector Structure") (L_Distance :type "Float (double-precision)"))
  (bind _particlesystem (`self.ParticleSystem`))
  (bind _returnvalue (+ (`local.L_Origin`) (* (`local.L_Direction`) (`local.L_Distance`))))
  (set `local.L_Origin` Origin)
  (set `local.L_Direction` Direction)
  (set `local.L_Distance` Distance)
  (bind (_outhit _returnvalue_2) (`KismetSystemLibrary.LineTraceSingle` :`End` _returnvalue :`TraceChannel` "TraceTypeQuery1" :`bTraceComplex` true :`DrawTime` 0.1))
  (`ParticleSystemComponent.SetBeamSourcePoint` _particlesystem 0 (`local.L_Origin`) 0)
  (if _returnvalue_2
    (bind (_bblockinghit _binitialoverlap _time _distance _location _impactpoint _normal _impactnormal _physmat _hitactor _hitcomponent _hitbonename _hititem _faceindex) (`GameplayStatics.BreakHitResult` _outhit))
    (`ParticleSystemComponent.SetBeamTargetPoint` _particlesystem 0 _impactpoint 0)
    (bind (_sectionindex _returnvalue_3) (`PrimitiveComponent.GetMaterialFromCollisionFaceIndex` _hitcomponent _faceindex))
    (if (== _returnvalue_3 "/Game/Materials/Mat_LaserReceiver.Mat_LaserReceiver")
      (message `/Game/Blueprints/Player/LaserState.ToggleState` _hitactor true)
      (elif (== _returnvalue_3 "/Game/Materials/Mat_LaserRefractor.Mat_LaserRefractor")
        (message `/Game/Blueprints/Player/LaserState.ToggleState` _hitactor true)))
    (else
      (`ParticleSystemComponent.SetBeamTargetPoint` _particlesystem 0 _returnvalue 0))))

(fn `UserConstructionScript`)