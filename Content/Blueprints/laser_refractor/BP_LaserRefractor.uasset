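; Laser refractor actor that, once switched on via ToggleState, emits its own beam and can pass activation along a chain of refractors and receivers.
; While on, Tick line-traces from Arrow1 and stretches the Lasersystem1 beam to the impact point or max distance.
; Hit faces with the receiver or refractor material send a toggle-on message to their actor.
; A one-second Delay in Tick then switches it off unless LaserStaysOn is set.
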(event `/Game/Blueprints/Player/LaserState.ToggleState`
  (params (`On/Off` :type Boolean))
  (set `self.isOn` `On/Off`)
  (`SceneComponent.SetVisibility` (`self.lasersystem1`) true false))

(event `self.ReceiveTick`
  (params (DeltaSeconds :type "Float (single-precision)"))
  (bind _arrow1 (`self.Arrow1`))
  (if (`self.isOn`)
    (`self.Cast Light` (`SceneComponent.K2_GetComponentLocation` _arrow1) (`SceneComponent.GetForwardVector` _arrow1) (`self.Max Distance Laser`))
    (`KismetSystemLibrary.Delay` 1.0)
    (if (`self.laser stays on`)
      (`SceneComponent.SetVisibility` (`self.lasersystem1`) true false)
      (set `self.isOn` true)
      (else
        (`SceneComponent.SetVisibility` (`self.lasersystem1`) false false)
        (set `self.isOn` false)))))

(fn `Cast Light`
  (params (origin :type "Vector Structure") (direction :type "Vector Structure") (distance :type "Float (double-precision)"))
  (locals (L_Origin :type "Vector Structure") (L_Direction :type "Vector Structure") (L_Distance :type "Float (double-precision)"))
  (bind _l_origin (`local.L_Origin`))
  (bind _returnvalue (+ _l_origin (* (`local.L_Direction`) (`local.L_Distance`))))
  (set `local.L_Origin` origin)
  (set `local.L_Direction` direction)
  (set `local.L_Distance` distance)
  (bind (_outhit _returnvalue_2) (`KismetSystemLibrary.LineTraceSingle` :`Start` _l_origin :`End` _returnvalue :`TraceChannel` "TraceTypeQuery1" :`bTraceComplex` true :`DrawTime` 0.1))
  (`ParticleSystemComponent.SetBeamSourcePoint` (`self.lasersystem1`) 0 (`local.L_Origin`) 0)
  (if _returnvalue_2
    (bind (_bblockinghit _binitialoverlap _time _distance _location _impactpoint _normal _impactnormal _physmat _hitactor _hitcomponent _hitbonename _hititem _faceindex) (`GameplayStatics.BreakHitResult` _outhit))
    (`ParticleSystemComponent.SetBeamTargetPoint` (`self.lasersystem1`) 0 _impactpoint 0)
    (bind (_sectionindex _returnvalue_3) (`PrimitiveComponent.GetMaterialFromCollisionFaceIndex` _hitcomponent _faceindex))
    (if (== _returnvalue_3 "/Game/Materials/Mat_LaserReceiver.Mat_LaserReceiver")
      (message `/Game/Blueprints/Player/LaserState.ToggleState` _hitactor true)
      (elif (== _returnvalue_3 "/Game/Materials/Mat_LaserRefractor.Mat_LaserRefractor")
        (message `/Game/Blueprints/Player/LaserState.ToggleState` _hitactor true)))
    (else
      (`ParticleSystemComponent.SetBeamTargetPoint` (`self.lasersystem1`) 0 _returnvalue 0))))

(fn `UserConstructionScript`
  (`parent.UserConstructionScript`))