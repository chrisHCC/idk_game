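; Moving platform Blueprint that uses an InterpToMovement component to travel between relative points PointA and PointB.
; The construction script builds the component's control points from those two variables.
; BeginPlay backs up both points, FREEZEPLATFORM sets both to a given position, and UnfreezePlatform restores the backups.
; Freeze and unfreeze only write the variables, without rebuilding the control points in this graph.
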(event `self.ReceiveBeginPlay`
  (set `self.PointAA` (`self.PointA`))
  (set `self.PointBB` (`self.PointB`)))

(event `FREEZEPLATFORM`
  (params (Position :type "Vector Structure"))
  (set `self.PointA` Position)
  (set `self.PointB` Position))

(event `UnfreezePlatform`
  (set `self.PointA` (`self.PointAA`))
  (set `self.PointB` (`self.PointBB`)))

(fn `UserConstructionScript`
  (set `InterpToMovementComponent.ControlPoints` (`|MakeArray` (make `InterpControlPoint` (`self.PointA`)) (make `InterpControlPoint` (`self.PointB`)) (struct) (struct)) (`self.InterpToMovement`)))