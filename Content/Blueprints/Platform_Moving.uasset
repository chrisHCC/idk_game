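; Moving platform actor that travels along relative control points using an InterpToMovement component.
; The construction script builds the component's control point list from the PointA, PointB and PointC variables.
; BeginPlay activates a NavigationInvoker component, and the movement itself is left to InterpToMovement with no Tick logic.
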(event `self.ReceiveBeginPlay`
  (`ActorComponent.Activate` (`self.NavigationInvoker`) false))

(fn `UserConstructionScript`
  (set `InterpToMovementComponent.ControlPoints` (`|MakeArray` (make `InterpControlPoint` (`self.PointA`)) (make `InterpControlPoint` (`self.PointB`)) (make `InterpControlPoint` (`self.PointC`)) (struct)) (`self.InterpToMovement`)))