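; Conveyor belt Blueprint that carries actors overlapping its Box along the reverse of the belt mesh's forward vector.
; While active, Tick moves them with unswept world offsets scaled by belt speed and delta time.
; A DoOnce passes scaled speed to the material's Speed parameter on the first active tick only.
; ToggleState switches the active flag without updating the material.
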(event `self.ReceiveTick`
  (params (DeltaSeconds :type "Float (single-precision)"))
  (if (`self.Starts without Activation`)
    (`|ExecutionSequence`
      (:`then_0`
        (for _array_element (`PrimitiveComponent.GetOverlappingActors` (`self.Box`) null)
          (`self.K2_AddActorWorldOffset` _array_element (* (* (`KismetMathLibrary.GetForwardVector` (`SceneComponent.K2_GetComponentRotation` (`self.ConverbeltGames`))) -1.0) (* DeltaSeconds (`self.Speed of Conveyor`))) false false)))
      (:`then_1`
        (`/Engine/EditorBlueprintResources/StandardMacros.DoOnce` false
          (:`Completed`
            (`MeshComponent.SetVectorParameterValueOnMaterials` (`self.ConverbeltGames`) "Speed" (`KismetMathLibrary.MakeVector` 0.0 (/ (`self.Speed of Conveyor`) 130.0)))))))))

(event `/Game/Blueprints/Player/LaserState.ToggleState`
  (params (`On/Off` :type Boolean))
  (set `self.Starts without Activation` `On/Off`))

(fn `UserConstructionScript`)