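; BP_AUDIOLOG is an audio log pickup that a VR motion controller collects by touch.
; It applies a selectable mesh on BeginPlay, and when its box overlaps a BP_MotionController it destroys itself and plays its chosen sound at the world origin.
; A PLAY function does the same in reverse order, while a separate PlaySound event destroys the actor and plays a fixed beep instead.
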(event `self.ReceiveBeginPlay`
  (`StaticMeshComponent.SetStaticMesh` (`self.StaticMesh`) (`self.SelectMesh`)))

(event `self.Box.OnComponentBeginOverlap`
  (params (OverlappedComponent :type "PrimitiveComponent Object Reference") (OtherActor :type "Actor Object Reference") (OtherComp :type "PrimitiveComponent Object Reference") (OtherBodyIndex :type Integer) (bFromSweep :type Boolean) (SweepResult :type "HitResult Structure (by ref)"))
  (cast `/Game/Blueprints/Player/BP_MotionController` OtherActor)
  (`self.K2_DestroyActor` self)
  (`GameplayStatics.PlaySoundAtLocation` (`self.SoundtoPlay`) (0.0 0.0 0.0) (struct) 1.0 1.0 0.0 null null null))

(event `/Game/Blueprints/Sound.PlaySound`
  (`self.K2_DestroyActor` self)
  (`GameplayStatics.PlaySoundAtLocation` "/Game/Audio/Music/beep-01a.beep-01a" (0.0 0.0 0.0) (struct) 1.0 1.0 0.0 null null null))

(fn `PLAY`
  (`GameplayStatics.PlaySoundAtLocation` (`self.SoundtoPlay`) (0.0 0.0 0.0) (struct) 1.0 1.0 0.0 null null null)
  (`self.K2_DestroyActor` self))

(fn `UserConstructionScript`)