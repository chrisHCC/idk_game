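; A sweeping laser hazard that restarts the current level when its beam hits a BP_levelMenu actor.
; After a short Delay on Tick, it line-traces from the arrow and stretches a particle beam to the impact or max range.
; A lethal hit starts a dark red camera fade and immediately reopens the level; the BP_LaserRefractor check is empty.
; The base mesh rotates each pass, flipping speed when world yaw leaves the min/max angles.
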(event `self.ReceiveTick`
  (params (DeltaSeconds :type "Float (single-precision)"))
  (bind _arrow (`self.Arrow`))
  (bind _sm_laser_low_lascam_base_drum_low (`self.SM_Laser_Low_LasCam_Base_Drum_Low`))
  (bind _returnvalue (`SceneComponent.K2_GetComponentLocation` _arrow))
  (bind (_returnvalue_roll _returnvalue_pitch _returnvalue_yaw) (`KismetMathLibrary.BreakRotator` (`SceneComponent.K2_GetComponentRotation` _sm_laser_low_lascam_base_drum_low)))
  (bind _returnvalue_2 (+ _returnvalue (* (`KismetMathLibrary.GetForwardVector` (`SceneComponent.K2_GetComponentRotation` _arrow)) (`self.Max Distance Laser`))))
  (`KismetSystemLibrary.Delay` 0.01)
  (`|ExecutionSequence`
    (:`then_0`
      (bind (_outhit _returnvalue_3) (`KismetSystemLibrary.LineTraceSingle` :`Start` _returnvalue :`End` _returnvalue_2 :`TraceChannel` "TraceTypeQuery1" :`DrawDebugType` "ForOneFrame"))
      (`ParticleSystemComponent.SetBeamSourcePoint` (`self.ParticleSystem`) 0 _returnvalue 0)
      (if _returnvalue_3
        (bind (_bblockinghit _binitialoverlap _time _distance _location _impactpoint _normal _impactnormal _physmat _hitactor) (`GameplayStatics.BreakHitResult` _outhit))
        (`ParticleSystemComponent.SetBeamTargetPoint` (`self.ParticleSystem`) 0 _impactpoint 0)
        (`|ExecutionSequence`
          (:`then_0`
            (bind _returnvalue_4 (`GameplayStatics.GetObjectClass` _hitactor))
            (if (== _returnvalue_4 "/Game/Blueprints/Widgets/BP_levelMenu.BP_levelMenu_C")
              (`|ExecutionSequence`
                (:`then_0`
                  (`PlayerCameraManager.StartCameraFade` (`GameplayStatics.GetPlayerCameraManager` 0) 0.0 1.0 0.1 (struct :`R` 0.151042 :`G` 0.00236 :`B` 0.008272 :`A` 1.0) false false))
                (:`then_1`
                  (bind _returnvalue_5 (`GameplayStatics.GetCurrentLevelName` true))
                  (`GameplayStatics.OpenLevel` (`KismetStringLibrary.Conv_StringToName` _returnvalue_5))))))
          (:`then_1`
            (if (== _returnvalue_4 "/Game/Blueprints/PickUpObjects/BP_LaserRefractor.BP_LaserRefractor_C")
              _)))
        (else
          (`ParticleSystemComponent.SetBeamTargetPoint` (`self.ParticleSystem`) 0 _returnvalue_2 0))))
    (:`then_1`
      (`SceneComponent.K2_AddLocalRotation` _sm_laser_low_lascam_base_drum_low (`KismetMathLibrary.MakeRotator` 0.0 0.0 (`self.Speed`)) false false)
      (`KismetSystemLibrary.PrintString` (`KismetStringLibrary.Conv_DoubleToString` _returnvalue_yaw))
      (if (> _returnvalue_yaw (`self.MaxAngle`))
        (set `self.Speed` (* (`self.Speed`) -1.0))
        (elif (< _returnvalue_yaw (`self.MinAngle`))
          (set `self.Speed` (* (`self.Speed`) -1.0)))))))

(fn `UserConstructionScript`)