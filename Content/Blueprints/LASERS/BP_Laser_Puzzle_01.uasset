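; Laser puzzle emitter that fires a beam along its arrow and switches on receiver actors it hits.
; Tick repeatedly calls CastLight after a short Delay, resetting the last activated sensor and looping visibility traces with beam particles.
; Complex traces read the hit face's material: refractor mirrors the direction and spawns another beam segment, while receiver sends ToggleStateMessage to its actor and ends the loop.
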(event `self.ReceiveTick`
  (params (DeltaSeconds :type "Float (single-precision)"))
  (bind _arrow (`self.Arrow`))
  (`|ExecutionSequence`
    (:`then_0`
      (`KismetSystemLibrary.Delay` 0.01)
      (`self.CastLight` (`SceneComponent.K2_GetComponentLocation` _arrow) (`SceneComponent.GetForwardVector` _arrow) (`self.Max Distance Laser`)))))

(fn `CastLight`
  (params (Origin :type "Vector Structure") (Direction :type "Vector Structure") (Distance :type "Float (double-precision)"))
  (locals (L_Origin :type "Vector Structure") (L_Direction :type "Vector Structure") (L_Distance :type "Float (double-precision)" :default 10000.0) (L_Continue :type Boolean :default true) (L_BeamStart :type "Vector Structure") (L_BeamEnd :type "Vector Structure") (prev :type Boolean))
  (bind _l_origin (`local.L_Origin`))
  (bind _returnvalue (+ _l_origin (* (`local.L_Direction`) (`local.L_Distance`))))
  (set `local.L_Origin` Origin)
  (set `local.L_Direction` Direction)
  (set `local.L_Distance` Distance)
  (message `/Game/Blueprints/LaserState.ToggleState` (`self.ActivatedSensor`) false)
  (while (`local.L_Continue`)
    (bind (_outhit _returnvalue_2) (`KismetSystemLibrary.LineTraceSingle` :`Start` _l_origin :`End` _returnvalue :`TraceChannel` "TraceTypeQuery1" :`bTraceComplex` true :`DrawDebugType` "ForOneFrame" :`DrawTime` 0.1))
    (`ParticleSystemComponent.SetBeamSourcePoint` (`self.ParticleSystem`) 0 (`local.L_Origin`) 0)
    (if _returnvalue_2
      (bind (_bblockinghit _binitialoverlap _time _distance _location _impactpoint _normal _impactnormal _physmat _hitactor _hitcomponent _hitbonename _hititem _faceindex) (`GameplayStatics.BreakHitResult` _outhit))
      (`ParticleSystemComponent.SetBeamTargetPoint` (`self.ParticleSystem`) 0 _impactpoint 0)
      (bind (_sectionindex _returnvalue_3) (`PrimitiveComponent.GetMaterialFromCollisionFaceIndex` _hitcomponent _faceindex))
      (if (== _returnvalue_3 "/Game/Materials/Mat_LaserRefractor.Mat_LaserRefractor")
        (bind _returnvalue_4 (`GameplayStatics.SpawnEmitterAtLocation` "/Game/Blueprints/laser_mat/lasersystem1.lasersystem1" (`local.L_Origin`)))
        (`ParticleSystemComponent.SetBeamSourcePoint` _returnvalue_4 0 (`local.L_Origin`) 0)
        (`ParticleSystemComponent.SetBeamTargetPoint` _returnvalue_4 0 _impactpoint 0)
        (set `local.L_Origin` _impactpoint)
        (set `local.L_Direction` (`KismetMathLibrary.MirrorVectorByNormal` (`local.L_Direction`) _impactnormal))
        (set `local.L_Continue` true)
        (else
          (if (== _returnvalue_3 "/Game/Materials/Mat_LaserReceiver.Mat_LaserReceiver")
            (`ParticleSystemComponent.SetBeamSourcePoint` _returnvalue_4 0 (`local.L_Origin`) 0)
            (`ParticleSystemComponent.SetBeamTargetPoint` _returnvalue_4 0 _impactpoint 0)
            (message `/Game/Blueprints/LaserState.ToggleState` _hitactor true)
            (set `self.ActivatedSensor` _hitactor))
          (set `local.L_Continue` false)))
      (else
        (`ParticleSystemComponent.SetBeamTargetPoint` (`self.ParticleSystem`) 0 _returnvalue 0)
        (set `local.L_Continue` false)
        (`ActorComponent.K2_DestroyComponent` _returnvalue_4)))))

(fn `UserConstructionScript`)