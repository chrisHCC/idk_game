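; BP_Laser1 is a laser hazard that restarts the current level when anything blocks its line.
; BeginPlay stretches a beam particle between two scene components, Scene and Scene1.
; Tick runs a debug-drawn Visibility trace between them; any hit starts a brief dark red camera fade, reopens the level and moves the beam end to the impact point.
; The hit is not filtered to the player.
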(event `self.ReceiveBeginPlay`
  (`ParticleSystemComponent.SetBeamSourcePoint` (`self.ParticleSystem`) 0 (`SceneComponent.K2_GetComponentLocation` (`self.Scene`)) 0)
  (`ParticleSystemComponent.SetBeamTargetPoint` (`self.ParticleSystem`) 0 (`SceneComponent.K2_GetComponentLocation` (`self.Scene1`)) 0))

(event `self.ReceiveTick`
  (params (DeltaSeconds :type "Float (single-precision)"))
  (bind (_outhit _returnvalue) (`KismetSystemLibrary.LineTraceSingle` :`Start` (`SceneComponent.K2_GetComponentLocation` (`self.Scene`)) :`End` (`SceneComponent.K2_GetComponentLocation` (`self.Scene1`)) :`TraceChannel` "TraceTypeQuery1" :`DrawDebugType` "ForOneFrame"))
  (if _returnvalue
    (`|ExecutionSequence`
      (:`then_0`
        (`PlayerCameraManager.StartCameraFade` (`GameplayStatics.GetPlayerCameraManager` 0) 0.0 1.0 0.1 (struct :`R` 0.151042 :`G` 0.00236 :`B` 0.008272 :`A` 1.0) false false))
      (:`then_1`
        (bind _returnvalue_2 (`GameplayStatics.GetCurrentLevelName` true))
        (`GameplayStatics.OpenLevel` (`KismetStringLibrary.Conv_StringToName` _returnvalue_2)))
      (:`then_2`
        (`ParticleSystemComponent.SetBeamTargetPoint` (`self.ParticleSystem`) 0 (`.ImpactPoint` (`GameplayStatics.BreakHitResult` _outhit)) 0)))))

(fn `UserConstructionScript`)