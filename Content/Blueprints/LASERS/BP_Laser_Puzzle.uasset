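; Laser emitter for a puzzle that fires a beam along its Arrow component and activates the refractors and receivers it hits.
; Tick, throttled by a short Delay, calls CastLight, which runs a complex Visibility line trace and sets the particle beam's endpoints.
; Targets are identified by the material at the hit face, and matching actors receive ToggleStateMessage(true); this Blueprint never sends false.
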(event `self.ReceiveTick`
  (params (DeltaSeconds :type "Float (single-precision)"))
  (bind _arrow (`self.Arrow`))
  (`|ExecutionSequence`
    (:`then_0`
      (`KismetSystemLibrary.Delay` 0.01)
      (`self.CastLight` (`SceneComponent.K2_GetComponentLocation` _arrow) (`SceneComponent.GetForwardVector` _arrow) (`self.Max Distance Laser`)))))

(fn `CastLight`
  (params (Origin :type "Vector Structure") (Direction :type "Vector Structure") (Distance :type "Float (double-precision)"))
  (locals (L_Origin :type "Vector Structure") (L_Direction :type "Vector Structure") (L_Distance :type "Float (double-precision)" :default 10000.0) (L_Continue :type Boolean :default true) (L_BeamStart :type "Vector Structure") (L_BeamEnd :type "Vector Structure") (prev :type Boolean))
  (bind _l_origin (`local.L_Origin`))
  (bind _returnvalue (+ _l_origin (* (`local.L_Direction`) (`local.L_Distance`))))
  (set `local.L_Origin` Origin)
  (set `local.L_Direction` Direction)
  (set `local.L_Distance` Distance)
  (bind (_outhit _returnvalue_2) (`KismetSystemLibrary.LineTraceSingle` :`Start` _l_origin :`End` _returnvalue :`TraceChannel` "TraceTypeQuery1" :`bTraceComplex` true :`DrawTime` 0.1))
  (`ParticleSystemComponent.SetBeamSourcePoint` (`self.ParticleSystem`) 0 (`local.L_Origin`) 0)
  (if _returnvalue_2
    (bind (_bblockinghit _binitialoverlap _time _distance _location _impactpoint _normal _impactnormal _physmat _hitactor _hitcomponent _hitbonename _hititem _faceindex) (`GameplayStatics.BreakHitResult` _outhit))
    (`ParticleSystemComponent.SetBeamTargetPoint` (`self.ParticleSystem`) 0 _impactpoint 0)
    (bind (_sectionindex _returnvalue_3) (`PrimitiveComponent.GetMaterialFromCollisionFaceIndex` _hitcomponent _faceindex))
    (if (== _returnvalue_3 "/Game/Materials/Mat_LaserRefractor.Mat_LaserRefractor")
      (message `/Game/Blueprints/LaserState.ToggleState` _hitactor true)
      (elif (== _returnvalue_3 "/Game/Materials/Mat_LaserReceiver.Mat_LaserReceiver")
        (message `/Game/Blueprints/LaserState.ToggleState` _hitactor true)))
    (else
      (`ParticleSystemComponent.SetBeamTargetPoint` (`self.ParticleSystem`) 0 _returnvalue 0))))

(fn `UserConstructionScript`)