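; BP_BELTCONV is a conveyor belt actor that carries whatever actors sit on it.
; Each Tick it gets the actors overlapping its Box and offsets them along the reversed forward vector of the ConverbeltGames component.
; The offset is scaled by SpeedOfConveyor and delta time and applied without sweep, so it moves actors directly rather than through physics.
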(event `self.ReceiveTick`
  (params (DeltaSeconds :type "Float (single-precision)"))
  (for _array_element (`PrimitiveComponent.GetOverlappingActors` (`self.Box`) null)
    (`self.K2_AddActorWorldOffset` _array_element (* (* (`KismetMathLibrary.GetForwardVector` (`SceneComponent.K2_GetComponentRotation` (`self.ConverbeltGames`))) -1.0) (* DeltaSeconds (`self.Speed of Conveyor`))) false false)))

(fn `UserConstructionScript`)