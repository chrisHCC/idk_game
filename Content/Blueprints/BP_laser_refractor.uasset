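; BP_laser_refractor is a laser refractor prop that a motion controller can pick up and drop.
; Pickup attaches it to the controller and Drop detaches it, both leaving mesh physics simulation off.
; Activated sets IsOn, after which Tick runs a one-unit forward debug line trace from the Scene component, with its result unused.
; A Box hit with initial overlap only prints a test message.
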(event `/Game/Blueprints/Player/PickupActorInterface.Pickup`
  (params (AttachTo :type "SceneComponent Object Reference"))
  (`PrimitiveComponent.SetSimulatePhysics` (`self.SM_Laser_Refractor_Low`) false)
  (`SceneComponent.K2_AttachToComponent` (`self.K2_GetRootComponent`) AttachTo "None" "KeepWorld" "KeepWorld" "KeepWorld" false))

(event `/Game/Blueprints/Player/PickupActorInterface.Drop`
  (`PrimitiveComponent.SetSimulatePhysics` (`self.SM_Laser_Refractor_Low`) false)
  (`self.K2_DetachFromActor` "KeepWorld" "KeepWorld" "KeepWorld"))

(event `self.ReceiveTick`
  (params (DeltaSeconds :type "Float (single-precision)"))
  (bind _scene (`self.Scene`))
  (bind _returnvalue (`SceneComponent.K2_GetComponentLocation` _scene))
  (if (`self.isOn?`)
    (`KismetSystemLibrary.LineTraceSingle` :`Start` _returnvalue :`End` (+ (`SceneComponent.GetForwardVector` _scene) _returnvalue) :`TraceChannel` "TraceTypeQuery1" :`DrawDebugType` "ForOneFrame")))

(event `Activated`
  (set `self.isOn?` true))

(event `self.Box.OnComponentHit`
  (params (HitComponent :type "PrimitiveComponent Object Reference") (OtherActor :type "Actor Object Reference") (OtherComp :type "PrimitiveComponent Object Reference") (NormalImpulse :type "Vector Structure") (Hit :type "HitResult Structure (by ref)"))
  (if (`.bInitialOverlap` (`GameplayStatics.BreakHitResult` Hit))
    (`KismetSystemLibrary.PrintString` "Hello")))

(fn `UserConstructionScript`)