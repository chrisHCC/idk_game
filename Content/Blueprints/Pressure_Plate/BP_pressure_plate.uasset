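; Pressure plate puzzle trigger that responds when a BP_PickupCube enters or leaves its box.
; Timelines lerp the pad between its start height and a Z offset, swapping on/off materials on pad and frame when finished.
; Entering sends ToggleStateMessage(true) to every AffectedActors entry.
; Leaving sends false without its own loop, reusing the entry loop's array element.
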(event `self.ReceiveBeginPlay`
  (bind _sm_presureplate_presurepad_low (`self.SM_PresurePlate_PresurePad_low`))
  (bind (_relativelocation_x _relativelocation_y _relativelocation_z) (`KismetMathLibrary.BreakVector` (`SceneComponent.RelativeLocation` _sm_presureplate_presurepad_low)))
  (set `self.InitialLocation` (`SceneComponent.RelativeLocation` _sm_presureplate_presurepad_low))
  (set `self.TargetLocation` (`KismetMathLibrary.MakeVector` _relativelocation_x _relativelocation_y (+ _relativelocation_z (`self.Z`)))))

(event `MoveDown`
  (bind (_direction _alpha) (`Timeline|Timeline_0` :!via `PlayFromStart`)
    (:`Update`
      (`SceneComponent.K2_SetRelativeLocation` (`self.SM_PresurePlate_PresurePad_low`) (`KismetMathLibrary.VLerp` (`self.InitialLocation`) (`self.TargetLocation`) _alpha) false false))
    (:`Finished`
      (`PrimitiveComponent.SetMaterial` (`self.SM_PresurePlate_PresureFrame_low`) 0 "/Game/Materials/Mat_presurePateOn.Mat_presurePateOn")
      (`PrimitiveComponent.SetMaterial` (`self.SM_PresurePlate_PresurePad_low`) 0 "/Game/Materials/Mat_presurePateOn.Mat_presurePateOn"))))

(event `self.Box.OnComponentBeginOverlap`
  (params (OverlappedComponent :type "PrimitiveComponent Object Reference") (OtherActor :type "Actor Object Reference") (OtherComp :type "PrimitiveComponent Object Reference") (OtherBodyIndex :type Integer) (bFromSweep :type Boolean) (SweepResult :type "HitResult Structure (by ref)"))
  (cast `/Game/Blueprints/BP_PickupCube` OtherActor)
  (`self.MoveDown`)
  (for _array_element (`self.AffectedActors`)
    (set `self.Activated` true)
    (message `/Game/Blueprints/LaserState.ToggleState` _array_element true)))

(event `self.Box.OnComponentEndOverlap`
  (params (OverlappedComponent :type "PrimitiveComponent Object Reference") (OtherActor :type "Actor Object Reference") (OtherComp :type "PrimitiveComponent Object Reference") (OtherBodyIndex :type Integer))
  (cast `/Game/Blueprints/BP_PickupCube` OtherActor)
  (`self.MoveUp`)
  (set `self.Activated` false)
  (message `/Game/Blueprints/LaserState.ToggleState` (stale `self.Box.OnComponentBeginOverlap` _array_element) false))

(event `MoveUp`
  (bind (_direction _alpha) (`Timeline|Timeline_1` :!via `PlayFromStart`)
    (:`Update`
      (`SceneComponent.K2_SetRelativeLocation` (`self.SM_PresurePlate_PresurePad_low`) (`KismetMathLibrary.VLerp` (`self.TargetLocation`) (`self.InitialLocation`) _alpha) false false))
    (:`Finished`
      (`PrimitiveComponent.SetMaterial` (`self.SM_PresurePlate_PresureFrame_low`) 0 "/Game/Materials/Mat_presurePlateOff.Mat_presurePlateOff")
      (`PrimitiveComponent.SetMaterial` (`self.SM_PresurePlate_PresurePad_low`) 0 "/Game/Materials/Mat_presurePlateOff.Mat_presurePlateOff"))))

(fn `UserConstructionScript`)