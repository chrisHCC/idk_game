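; Wall-mounted pressure plate that captures an overlapping BP_PickupCube whose scale roughly matches WantedScale and switches on linked actors.
; A match makes the player's gun drop the cube, starts a timeline gliding it to a snap transform built at BeginPlay, and immediately sends ToggleStateMessage to AffectedActors.
; Once the timeline finishes, Tick pins the cube there and sets its mobility to Stationary once.
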(event `self.ReceiveBeginPlay`
  (bind _returnvalue_location (`KismetMathLibrary.BreakTransform` (`SceneComponent.K2_GetComponentToWorld` (`self.Scene`))))
  (bind (_returnvalue_roll _returnvalue_pitch _returnvalue_yaw) (`KismetMathLibrary.BreakRotator` (`SceneComponent.K2_GetComponentRotation` (`self.SM_PresurePlate_PresureFrame_low`))))
  (bind _output_get (set `self.Snap Location` (`KismetMathLibrary.MakeTransform` _returnvalue_location (`KismetMathLibrary.MakeRotator` _returnvalue_roll (+ _returnvalue_pitch 90.0) _returnvalue_yaw)))))

(event `animation`
  (bind (_direction _alpha) (`Timeline|Timeline_0`)
    (:`Update`
      (`SceneComponent.K2_SetWorldTransform` (`Actor.RootComponent` (stale `self.Box.OnComponentBeginOverlap` _asbp_pickup_cube)) (`KismetMathLibrary.TLerp` (`self.Grabed Location`) (`self.Snap Location`) _alpha) false false))
    (:`Finished`
      (set `self.Snap` true))))

(event `self.ReceiveTick`
  (params (DeltaSeconds :type "Float (single-precision)"))
  (if (`self.Snap`)
    (bind _rootcomponent (`Actor.RootComponent` (stale `self.Box.OnComponentBeginOverlap` _asbp_pickup_cube)))
    (`SceneComponent.K2_SetWorldTransform` _rootcomponent (`self.Snap Location`) false false)
    (`/Engine/EditorBlueprintResources/StandardMacros.DoOnce` false
      (:`Completed`
        (`SceneComponent.SetMobility` _rootcomponent "Stationary")))))

(event `self.Box.OnComponentBeginOverlap`
  (params (OverlappedComponent :type "PrimitiveComponent Object Reference") (OtherActor :type "Actor Object Reference") (OtherComp :type "PrimitiveComponent Object Reference") (OtherBodyIndex :type Integer) (bFromSweep :type Boolean) (SweepResult :type "HitResult Structure (by ref)"))
  (bind _asbp_pickup_cube (cast `/Game/Blueprints/Player/BP_PickupCube` OtherActor))
  (if (== (`/Game/Blueprints/Player/BP_PickupCube.Scale` _asbp_pickup_cube) (`self.Wanted Scale`) :`ErrorTolerance` 0.1)
    (set `self.Grabed Location` (`KismetMathLibrary.MakeTransform` (`self.K2_GetActorLocation` _asbp_pickup_cube) (.rotation (stale `self.ReceiveBeginPlay` _output_get))))
    (`/Game/Blueprints/Player/mcpawn.DropObjectinGun` (`self.McPawn Ref`))
    (`self.animation`)
    (for _array_element (`self.AffectedActors`)
      (set `self.Activated` true)
      (message `/Game/Blueprints/Player/LaserState.ToggleState` _array_element true))))

(fn `UserConstructionScript`)