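; BP_DOOR_2 is a two-panel sliding door that opens when the player pawn enters its In trigger and closes on exit.
; After a one-second delay, timelines drive each panel's relative location to open, while closing uses separate reversed timelines that set both panels directly to zero.
; The blocking Box's collision toggles without waiting for movement.
; ToggleState exposes the same open/close logic for external control.
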(event `Open Door`
  (if (`self.Opening`)
    (`KismetSystemLibrary.Delay` 1.0)
    (`|ExecutionSequence`
      (:`then_0`
        (bind (_direction _newtrack_0) (`Timeline|Timeline_0`)
          (:`Update`
            (`SceneComponent.K2_SetRelativeLocation` (`self.SM_Door_low_SM_DoorLeft`) _newtrack_0 false false))))
      (:`then_1`
        (bind (_direction_2 _newtrack_0_2) (`Timeline|Timeline_1`)
          (:`Update`
            (`SceneComponent.K2_SetRelativeLocation` (`self.SM_Door_low_SM_DoorRight`) _newtrack_0_2 false false)))))))

(event `Close Door`
  (if (not (`self.Opening`))
    (`KismetSystemLibrary.Delay` 1.0)
    (`|ExecutionSequence`
      (:`then_0`
        (`Timeline|Timeline_2` :!via `Reverse`
          (:`Update`
            (`SceneComponent.K2_SetRelativeLocation` (`self.SM_Door_low_SM_DoorLeft`) (0.0 0.0 0.0) false false))))
      (:`then_1`
        (`Timeline|Timeline_3` :!via `Reverse`
          (:`Update`
            (`SceneComponent.K2_SetRelativeLocation` (`self.SM_Door_low_SM_DoorRight`) (0.0 0.0 0.0) false false)))))))

(event `self.In.OnComponentBeginOverlap`
  (params (OverlappedComponent :type "PrimitiveComponent Object Reference") (OtherActor :type "Actor Object Reference") (OtherComp :type "PrimitiveComponent Object Reference") (OtherBodyIndex :type Integer) (bFromSweep :type Boolean) (SweepResult :type "HitResult Structure (by ref)"))
  (bind _box (`self.Box`))
  (if (== OtherActor (`GameplayStatics.GetPlayerPawn` 0))
    (set `self.Opening` true)
    (`self.Open Door`)
    (set `PrimitiveComponent.CanCharacterStepUpOn` "ECB_Yes" _box :!label _label)
    (`PrimitiveComponent.SetCollisionEnabled` _box "NoCollision")))

(event `self.In.OnComponentEndOverlap`
  (params (OverlappedComponent :type "PrimitiveComponent Object Reference") (OtherActor :type "Actor Object Reference") (OtherComp :type "PrimitiveComponent Object Reference") (OtherBodyIndex :type Integer))
  (bind _box (`self.Box`))
  (if (== OtherActor (`GameplayStatics.GetPlayerPawn` 0))
    (set `self.Opening` false)
    (`self.Close Door`)
    (set `PrimitiveComponent.CanCharacterStepUpOn` "ECB_No" _box :!label _label_2)
    (`PrimitiveComponent.SetCollisionEnabled` _box "QueryAndPhysics")))

(event `/Game/Blueprints/Player/LaserState.ToggleState`
  (params (`On/Off` :type Boolean))
  (bind _output_get (set `self.Opening` `On/Off`))
  (if _output_get
    (`self.Open Door`)
    (goto _label)
    (else
      (`self.Close Door`)
      (goto _label_2))))

(fn `UserConstructionScript`)