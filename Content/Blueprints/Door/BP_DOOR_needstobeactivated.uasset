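; Two-panel sliding door Blueprint that opens or closes when activated through ToggleState, which stores the state in Opening.
; Opening waits a second, then two timelines drive the left and right panels' relative locations.
; Overlapping the Out component clears Opening and triggers closing.
; Closing waits a second and reverses two separate timelines, but their updates set both panels straight to zero relative location rather than interpolating.
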(event `Open Door`
  (`KismetSystemLibrary.Delay` 1.0)
  (`|ExecutionSequence`
    (:`then_0`
      (bind (_direction _newtrack_0) (`Timeline|Timeline_0`)
        (:`Update`
          (`SceneComponent.K2_SetRelativeLocation` (`self.SM_Door_low_SM_DoorLeft`) _newtrack_0 false false))))
    (:`then_1`
      (bind (_direction_2 _newtrack_0_2) (`Timeline|Timeline_1`)
        (:`Update`
          (`SceneComponent.K2_SetRelativeLocation` (`self.SM_Door_low_SM_DoorRight`) _newtrack_0_2 false false))))))

(event `Close Door`
  (if (not (`self.Opening`))
    (`KismetSystemLibrary.Delay` 1.0)
    (`|ExecutionSequence`
      (:`then_0`
        (`Timeline|Timeline_2` :!via `Reverse`
          (:`Update`
            (`SceneComponent.K2_SetRelativeLocation` (`self.SM_Door_low_SM_DoorLeft`) (0.0 0.0 0.0) false false))))
      (:`then_1`
        (`Timeline|Timeline_3` :!via `Reverse`
          (:`Update`
            (`SceneComponent.K2_SetRelativeLocation` (`self.SM_Door_low_SM_DoorRight`) (0.0 0.0 0.0) false false)))))))

(event `self.Out.OnComponentBeginOverlap`
  (params (OverlappedComponent :type "PrimitiveComponent Object Reference") (OtherActor :type "Actor Object Reference") (OtherComp :type "PrimitiveComponent Object Reference") (OtherBodyIndex :type Integer) (bFromSweep :type Boolean) (SweepResult :type "HitResult Structure (by ref)"))
  (set `self.Opening` false)
  (`self.Close Door`))

(event `/Game/Blueprints/LaserState.ToggleState`
  (params (`On/Off` :type Boolean))
  (bind _output_get (set `self.Opening` `On/Off`))
  (if _output_get
    (`self.Open Door`)
    (else
      (`self.Close Door`))))

(fn `UserConstructionScript`)