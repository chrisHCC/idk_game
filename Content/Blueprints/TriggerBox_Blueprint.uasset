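; Trigger box that shows whether the actor entering it is the object the player is currently holding.
; On BeginPlay it caches the first Mcpawn as the player and the first BP_PickupCube, though the cube reference is not used afterwards.
; When its collision component is overlapped, it compares the other actor to the player's HeldObjectRef and sets its text render to Good or Bad.
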(event `self.ReceiveBeginPlay`
  (bind _outactors (`GameplayStatics.GetAllActorsOfClass` "/Game/Blueprints/Player/mcpawn.mcpawn_C"))
  (set `self.PLAYER REF` (`|GetArrayItem` _outactors))
  (bind _outactors_2 (`GameplayStatics.GetAllActorsOfClass` "/Game/Blueprints/BP_PickupCube.BP_PickupCube_C"))
  (set `self.REF CUBE` (`|GetArrayItem` _outactors_2)))

(event `self.CollisionComponent.OnComponentBeginOverlap`
  (params (OverlappedComponent :type "PrimitiveComponent Object Reference") (OtherActor :type "Actor Object Reference") (OtherComp :type "PrimitiveComponent Object Reference") (OtherBodyIndex :type Integer) (bFromSweep :type Boolean) (SweepResult :type "HitResult Structure (by ref)"))
  (bind _textrender (`self.TextRender`))
  (if (== OtherActor (`/Game/Blueprints/Player/mcpawn.HeldObjectRef` (`self.PLAYER REF`)))
    (`TextRenderComponent.K2_SetText` _textrender (`self.good`))
    (else
      (`TextRenderComponent.K2_SetText` _textrender (`self.bad`)))))

(fn `UserConstructionScript`)