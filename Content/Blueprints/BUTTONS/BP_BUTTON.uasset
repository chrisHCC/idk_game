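; BP_BUTTON is a button actor whose Activate function sends ToggleStateMessage to every actor in AffectedActors.
; Separately, ToggleState and ANIMATION play a timeline that moves the top mesh from its BeginPlay location toward an XYZ offset.
; The offset is added to the mesh's current location each update.
; After a one-second delay the timeline reverses, with a DoOnce, reset on each trigger, preventing repeated reversals.
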(event `self.ReceiveBeginPlay`
  (set `self.savedInitialLocation` (`SceneComponent.K2_GetComponentLocation` (`self.SM_Button_ButtonTop_low`))))

(event `/Game/Blueprints/Player/LaserState.ToggleState`
  (params (`On/Off` :type Boolean))
  (bind _sm_button_buttontop_low (`self.SM_Button_ButtonTop_low`))
  (bind (_returnvalue_x _returnvalue_y _returnvalue_z) (`KismetMathLibrary.BreakVector` (`SceneComponent.K2_GetComponentLocation` _sm_button_buttontop_low)))
  (`|ExecutionSequence` :!label _label
    (:`then_0`
      (bind (_direction _alpha) (`Timeline|Timeline_0` :!via `PlayFromStart` :!label _label_2)
        (:`Update`
          (`SceneComponent.K2_SetWorldLocation` _sm_button_buttontop_low (`KismetMathLibrary.VLerp` (`self.savedInitialLocation`) (`KismetMathLibrary.MakeVector` (+ _returnvalue_x (`self.X`)) (+ _returnvalue_y (`self.Y`)) (+ _returnvalue_z (`self.Z`))) _alpha) false false))
        (:`Finished`
          (`KismetSystemLibrary.Delay` 1.0)
          (`/Engine/EditorBlueprintResources/StandardMacros.DoOnce` false :!label _label_3
            (:`Completed`
              (`self.Reverse`))))))
    (:`then_1`
      (goto _label_3 :!via `Reset`))))

(event `Reverse`
  (goto _label_2 :!via `ReverseFromEnd`))

(event `ANIMATION`
  (goto _label))

(fn `Activate`
  (for _array_element (`self.AffectedActors`)
    (message `/Game/Blueprints/Player/LaserState.ToggleState` _array_element true)))

(fn `UserConstructionScript`)