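; BP_BUTTON is a button actor that switches on other actors and can show a press motion.
; Activate loops through AffectedActors and sends each ToggleStateMessage with true.
; The separate ANIMATION event saves the button top's location, offsets it by the X, Y and Z variables, then restores it after a one-second delay.
; Both lerps use a fixed alpha of 1, so the top snaps between positions rather than sliding.
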(event `ANIMATION`
  (bind _sm_button_buttontop_low (`self.SM_Button_ButtonTop_low`))
  (bind _returnvalue (`SceneComponent.K2_GetComponentLocation` _sm_button_buttontop_low))
  (bind (_returnvalue_x _returnvalue_y _returnvalue_z) (`KismetMathLibrary.BreakVector` (`SceneComponent.K2_GetComponentLocation` _sm_button_buttontop_low)))
  (bind _returnvalue_2 (`KismetMathLibrary.MakeVector` (+ _returnvalue_x (`self.X`)) (+ _returnvalue_y (`self.Y`)) (+ _returnvalue_z (`self.Z`))))
  (set `self.savedInitialLocation` _returnvalue)
  (`SceneComponent.K2_SetWorldLocation` _sm_button_buttontop_low (`KismetMathLibrary.VLerp` _returnvalue _returnvalue_2 1.0) false false)
  (`KismetSystemLibrary.Delay` 1.0)
  (`SceneComponent.K2_SetWorldLocation` (`self.SM_Button_ButtonTop_low`) (`KismetMathLibrary.VLerp` _returnvalue_2 (`self.savedInitialLocation`) 1.0) false false))

(fn `Activate`
  (for _array_element (`self.AffectedActors`)
    (message `/Game/Blueprints/LaserState.ToggleState` _array_element true)))

(fn `UserConstructionScript`)