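; Teleporter actor that sends the player pawn to the next level when it overlaps the trigger box while activated.
; ToggleState switches it on or off.
; On overlap it fades the camera toward dark blue, plays a sound at the pawn, shows the loading screen, and after a short delay sets the target map on GI_main and calls ChangeMap.
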(event `/Game/Blueprints/Player/LaserState.ToggleState`
  (params (`On/Off` :type Boolean))
  (set `self.Activated?` `On/Off`))

(event `self.Box.OnComponentBeginOverlap`
  (params (OverlappedComponent :type "PrimitiveComponent Object Reference") (OtherActor :type "Actor Object Reference") (OtherComp :type "PrimitiveComponent Object Reference") (OtherBodyIndex :type Integer) (bFromSweep :type Boolean) (SweepResult :type "HitResult Structure (by ref)"))
  (if (`self.Activated?`)
    (bind _asmcpawn (cast `/Game/Blueprints/Player/mcpawn` OtherActor))
    (`PlayerCameraManager.StartCameraFade` (`GameplayStatics.GetPlayerCameraManager` 0) 0.0 0.5 1.0 (struct :`R` 0.01671 :`G` 0.055182 :`B` 0.291667 :`A` 1.0) false false)
    (`GameplayStatics.PlaySoundAtLocation` (`self.Select Sound:`) (`self.K2_GetActorLocation` _asmcpawn) (struct) 1.0 1.0 0.0 null null null)
    (`XRLoadingScreenFunctionLibrary.ShowLoadingScreen`)
    (`KismetSystemLibrary.Delay` 2.0)
    (bind _asgi_main (cast `/Game/Blueprints/Player/GI_main` (`GameplayStatics.GetGameInstance`)))
    (set `/Game/Blueprints/Player/GI_main.Map` (`self.Select Next Level`) _asgi_main)
    (`/Game/Blueprints/Player/GI_main.ChangeMap` _asgi_main)))

(fn `UserConstructionScript`)