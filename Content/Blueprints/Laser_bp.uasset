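; Rotating laser hazard that restarts the current level when its beam hits the player pawn or a VR motion controller.
; Each tick it spins the static mesh slightly and passes the Arrow's position, forward vector and cast distance to a trace function.
; While the Continue flag is set, that function runs a complex Visibility line trace with timed debug drawing and checks the hit actor's exact class.
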(event `self.ReceiveBeginPlay`
  (bind _asmcpawn (cast `/Game/Blueprints/Player/mcpawn` (`self.GetOwner`)))
  (set `self.mcRef` _asmcpawn))

(event `self.ReceiveTick`
  (params (DeltaSeconds :type "Float (single-precision)"))
  (bind _arrow (`self.Arrow`))
  (`SceneComponent.K2_AddLocalRotation` (`self.StaticMesh`) (struct :`Yaw` 0.1) false false)
  (`self.NewFunction_0` (`SceneComponent.K2_GetComponentLocation` _arrow) (`SceneComponent.GetForwardVector` _arrow) (`self.cast distance`)))

(fn `NewFunction_0`
  (params (location :type "Vector Structure") (direction :type "Vector Structure") (distance :type "Float (double-precision)"))
  (locals (origin :type "Vector Structure") (`cast d` :type "Vector Structure") (NewLocalVar_2 :type "Float (double-precision)" :default 1000.0) (continue :type Boolean :default true))
  (bind _origin (`local.origin`))
  (set `local.origin` location)
  (set `local.cast d` direction)
  (set `local.NewLocalVar_2` distance)
  (if (`local.continue`)
    (bind _outhit (`KismetSystemLibrary.LineTraceSingle` :`Start` _origin :`End` (+ _origin (* (`local.cast d`) (`local.NewLocalVar_2`))) :`TraceChannel` "TraceTypeQuery1" :`bTraceComplex` true :`DrawDebugType` "ForDuration" :`bIgnoreSelf` false :`DrawTime` 1.0))
    (bind (_bblockinghit _binitialoverlap _time _distance _location _impactpoint _normal _impactnormal _physmat _hitactor) (`GameplayStatics.BreakHitResult` _outhit))
    (if (or (== (`GameplayStatics.GetObjectClass` _hitactor) "/Game/Blueprints/Player/mcpawn.mcpawn_C") (== (`GameplayStatics.GetObjectClass` _hitactor) "/Game/Blueprints/Player/BP_MotionController.BP_MotionController_C"))
      (bind _returnvalue (`GameplayStatics.GetCurrentLevelName` true))
      (`GameplayStatics.OpenLevel` (`KismetStringLibrary.Conv_StringToName` _returnvalue)))
    (set `local.continue` true)))

(fn `UserConstructionScript`)