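; BP_scale is a toggle power-up that switches the scale ability on the player's mcpawn.
; On BeginPlay it casts player pawn 0 to mcpawn and caches the reference.
; ButtonAction calls ToggleScale on that pawn, then briefly flashes the power-up's name on a TextRender before hiding it again.
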(event `self.ReceiveBeginPlay`
  ;[1 1 1] cast to player / set player ref
  (bind _asmcpawn (cast `/Game/Blueprints/Player/mcpawn` (`GameplayStatics.GetPlayerPawn` 0)))
  (set `self.PlayerRef` _asmcpawn))

(event `self.ButtonAction`
  (bind _textrender (`self.TextRender`))
  ;[1 1 1] toogle scale in mcpawn
  (`/Game/Blueprints/Player/mcpawn.ToggleScale` (`self.playerref`))
  (`SceneComponent.SetVisibility` _textrender true false)
  (`TextRenderComponent.K2_SetText` _textrender (`self.NamePowerUp`))
  (`KismetSystemLibrary.Delay` 0.1)
  (`SceneComponent.SetVisibility` _textrender false false))

(fn `UserConstructionScript`
  (`parent.UserConstructionScript`))