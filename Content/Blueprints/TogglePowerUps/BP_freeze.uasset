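; Toggle power-up Blueprint that switches the freeze ability on the player pawn when its button action fires.
; On BeginPlay it casts the player pawn to mcpawn and caches the reference.
; The button action calls ToggleFreeze on that pawn, then shows the power-up name on a text render for half a second before hiding it.
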(event `self.ReceiveBeginPlay`
  ;[1 1 1] cast to player/ player reference
  (bind _asmcpawn (cast `/Game/Blueprints/Player/mcpawn` (`GameplayStatics.GetPlayerPawn` 0)))
  (set `self.playerref` _asmcpawn))

(event `self.ButtonAction`
  (bind _textrender (`self.TextRender`))
  ;[1 1 1] toggle scale / sets text to scale
  (`/Game/Blueprints/Player/mcpawn.ToggleFreeze` (`self.playerref`))
  (`SceneComponent.SetVisibility` _textrender true false)
  (`TextRenderComponent.K2_SetText` _textrender (`self.nameporwerup`))
  (`KismetSystemLibrary.Delay` 0.5)
  (`SceneComponent.SetVisibility` _textrender false false))

(fn `UserConstructionScript`
  (`parent.UserConstructionScript`))