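; BP_WeightChange is a toggle power-up actor that switches the player's mass.
; On BeginPlay it casts player pawn 0 to mcpawn and caches the reference.
; Its ButtonAction event calls ToggleMass on that pawn, then briefly flashes the power-up name on a text render component before hiding it again.
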(event `self.ReceiveBeginPlay`
  ;[1 1 1] cast to player/ player reference
  (bind _asmcpawn (cast `/Game/Blueprints/Player/mcpawn` (`GameplayStatics.GetPlayerPawn` 0)))
  (set `self.player ref` _asmcpawn))

(event `self.ButtonAction`
  (bind _textrender (`self.TextRender`))
  ;[1 1 1] toggle scale / sets text to scale
  (`/Game/Blueprints/Player/mcpawn.ToggleMass` (`self.player ref`))
  (`SceneComponent.SetVisibility` _textrender true false)
  (`TextRenderComponent.K2_SetText` _textrender (`self.namepowerup`))
  (`KismetSystemLibrary.Delay` 0.1)
  (`SceneComponent.SetVisibility` _textrender false false))

(fn `UserConstructionScript`
  (`parent.UserConstructionScript`))