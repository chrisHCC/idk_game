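; Base Blueprint for VR push buttons, pressed by the finger collision of a BP_MotionController overlapping its Box.
; An accepted press stores the fingertip and mesh start location, then calls ButtonAction, an empty function here.
; A DisablePress flag guards the press but is cleared immediately by ResetButton, and also when the finger leaves the Box.
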(event `self.ReceiveTick`
  (params (DeltaSeconds :type "Float (single-precision)")))

(event `self.Box.OnComponentBeginOverlap`
  (params (OverlappedComponent :type "PrimitiveComponent Object Reference") (OtherActor :type "Actor Object Reference") (OtherComp :type "PrimitiveComponent Object Reference") (OtherBodyIndex :type Integer) (bFromSweep :type Boolean) (SweepResult :type "HitResult Structure (by ref)"))
  (if (not (`self.Disable Press`))
    (bind _asbp_motion_controller (cast `/Game/Blueprints/Player/BP_MotionController` OtherActor))
    (bind _fingercollision (`/Game/Blueprints/Player/BP_MotionController.FingerCollision` _asbp_motion_controller))
    (if (== _fingercollision OtherComp)
      (set `self.Disable Press` true)
      (set `self.Finger Tip` _fingercollision)
      (set `self.Button Start Location` (`SceneComponent.RelativeLocation` (`self.StaticMesh`)))
      (`self.Button Action`)
      (`self.ResetButton`))))

(event `ResetButton`
  (set `self.Disable Press` false :!label _label))

(event `self.Box.OnComponentEndOverlap`
  (params (OverlappedComponent :type "PrimitiveComponent Object Reference") (OtherActor :type "Actor Object Reference") (OtherComp :type "PrimitiveComponent Object Reference") (OtherBodyIndex :type Integer))
  (bind _asbp_motion_controller (cast `/Game/Blueprints/Player/BP_MotionController` OtherActor))
  (if (== (`/Game/Blueprints/Player/BP_MotionController.FingerCollision` _asbp_motion_controller) OtherComp)
    (goto _label)))

(fn `Button Action`)

(fn `UserConstructionScript`)