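; BP_LASER_DEATH is a lethal laser that restarts the current level when its beam hits a BP_mapmenu actor.
; After a short Delay on Tick, it traces on Visibility from its Arrow and sets the particle beam's endpoints to the Arrow and the impact point or max range.
; A BP_mapmenu hit starts a dark-red camera fade and immediately reopens the level; the BP_laser_refractor check is empty.
; The drum mesh rotates slowly throughout.
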(event `self.ReceiveTick`
  (params (DeltaSeconds :type "Float (single-precision)"))
  (bind _arrow (`self.Arrow`))
  (bind _returnvalue (`SceneComponent.K2_GetComponentLocation` _arrow))
  (bind _returnvalue_2 (+ _returnvalue (* (`KismetMathLibrary.GetForwardVector` (`SceneComponent.K2_GetComponentRotation` _arrow)) (`self.Max Distance Laser`))))
  (`KismetSystemLibrary.Delay` 0.01)
  (`|ExecutionSequence`
    (:`then_0`
      (bind (_outhit _returnvalue_3) (`KismetSystemLibrary.LineTraceSingle` :`Start` _returnvalue :`End` _returnvalue_2 :`TraceChannel` "TraceTypeQuery1" :`DrawDebugType` "ForOneFrame"))
      (`ParticleSystemComponent.SetBeamSourcePoint` (`self.ParticleSystem`) 0 _returnvalue 0)
      (if _returnvalue_3
        (bind (_bblockinghit _binitialoverlap _time _distance _location _impactpoint _normal _impactnormal _physmat _hitactor) (`GameplayStatics.BreakHitResult` _outhit))
        (`ParticleSystemComponent.SetBeamTargetPoint` (`self.ParticleSystem`) 0 _impactpoint 0)
        (`|ExecutionSequence`
          (:`then_0`
            (bind _returnvalue_4 (`GameplayStatics.GetObjectClass` _hitactor))
            (if (== _returnvalue_4 "/Game/Blueprints/Widgets/BP_mapmenu.BP_mapmenu_C")
              (`|ExecutionSequence`
                (:`then_0`
                  (`PlayerCameraManager.StartCameraFade` (`GameplayStatics.GetPlayerCameraManager` 0) 0.0 1.0 0.1 (struct :`R` 0.151042 :`G` 0.00236 :`B` 0.008272 :`A` 1.0) false false))
                (:`then_1`
                  (bind _returnvalue_5 (`GameplayStatics.GetCurrentLevelName` true))
                  (`GameplayStatics.OpenLevel` (`KismetStringLibrary.Conv_StringToName` _returnvalue_5))))))
          (:`then_1`
            (if (== _returnvalue_4 "/Game/Blueprints/BP_laser_refractor.BP_laser_refractor_C")
              _)))
        (else
          (`ParticleSystemComponent.SetBeamTargetPoint` (`self.ParticleSystem`) 0 _returnvalue_2 0))))
    (:`then_1`
      (`SceneComponent.K2_AddLocalRotation` (`self.SM_Laser_Low_LasCam_Base_Drum_Low`) (struct :`Yaw` 0.1) false false))))

(fn `UserConstructionScript`)