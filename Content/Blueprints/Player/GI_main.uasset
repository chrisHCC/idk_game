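; GI_main, apparently the Game Instance going by its name, handles switching between the game's numbered levels.
; Its ChangeMap event switches on the Map value and opens the matching level by name, covering Level 1 through Level 17.
; A Map value of None falls back to the first level.
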(event `ChangeMap`
  (switch `/Game/Blueprints/Player/Map` (`self.Map`)
    (:`NewEnumerator0`
      (`GameplayStatics.OpenLevel` "Level_01" :!label _label))
    (:`NewEnumerator1`
      (goto _label))
    (:`NewEnumerator2`
      (`GameplayStatics.OpenLevel` "Level_02"))
    (:`NewEnumerator3`
      (`GameplayStatics.OpenLevel` "Level_03"))
    (:`NewEnumerator4`
      (`GameplayStatics.OpenLevel` "Level_04"))
    (:`NewEnumerator5`
      (`GameplayStatics.OpenLevel` "Level_05"))
    (:`NewEnumerator6`
      (`GameplayStatics.OpenLevel` "Level_06"))
    (:`NewEnumerator7`
      (`GameplayStatics.OpenLevel` "Level_07"))
    (:`NewEnumerator8`
      (`GameplayStatics.OpenLevel` "Level_08"))
    (:`NewEnumerator9`
      (`GameplayStatics.OpenLevel` "Level_09"))
    (:`NewEnumerator10`
      (`GameplayStatics.OpenLevel` "Level_10"))
    (:`NewEnumerator11`
      (`GameplayStatics.OpenLevel` "Level_11"))
    (:`NewEnumerator12`
      (`GameplayStatics.OpenLevel` "Level_12"))
    (:`NewEnumerator13`
      (`GameplayStatics.OpenLevel` "Level_13"))
    (:`NewEnumerator14`
      (`GameplayStatics.OpenLevel` "Level_14"))
    (:`NewEnumerator15`
      (`GameplayStatics.OpenLevel` "Level_15"))
    (:`NewEnumerator16`
      (`GameplayStatics.OpenLevel` "Level_16"))
    (:`NewEnumerator17`
      (`GameplayStatics.OpenLevel` "Level_17"))))