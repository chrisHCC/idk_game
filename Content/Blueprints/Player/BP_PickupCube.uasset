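; VR pickup cube that motion controllers grab and release, with floating control hints for the Launch, Freeze and Scale power-ups.
; Pickup, called by BP_MotionController, disables physics and attaches the cube to the given component; Drop reverses both.
; ToggleText picks a hint by headset and power-up, which the SHOW TEXT macro flashes briefly on TextRender.
; BeginPlay caches the starting scale, and ToggleState only sets the Frozen flag.
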(event `/Game/Blueprints/Player/LaserState.ToggleText`
  (params (powerUp :type "/Game/Blueprints/Player/E_ModeSelection Enum" :default "NewEnumerator0"))
  (bind _textrender (`self.TextRender`))
  (switch `name` (`HeadMountedDisplayFunctionLibrary.GetHMDDeviceName`)
    (:`Default`
      (switch `/Game/Blueprints/Player/E_ModeSelection` powerUp :!label _label
        (:`NewEnumerator0`
          (`self.SHOW TEXT` _textrender (`self.Trigger to Launch`) :!label _label_2))
        (:`NewEnumerator1`
          (`self.SHOW TEXT` _textrender (`self.Menu(R) toggle power ups`) :!label _label_3))
        (:`NewEnumerator2`
          (goto _label_3))))
    (:`OculusHMD`
      (switch `/Game/Blueprints/Player/E_ModeSelection` powerUp
        (:`NewEnumerator0`
          (`self.SHOW TEXT` _textrender (`self.Oculus (R) Grip to launch`)))
        (:`NewEnumerator1`
          (`self.SHOW TEXT` _textrender (`self.Oculus Press A`)))
        (:`NewEnumerator2`
          (`self.SHOW TEXT` _textrender (`self.Oculus Press B`)))
        (:`NewEnumerator4`
          (`self.SHOW TEXT` _textrender (`self.Oculus Right Trigger to Grab`)))))
    (:`SteamVR`
      (switch `/Game/Blueprints/Player/E_ModeSelection` powerUp
        (:`NewEnumerator0`
          (goto _label_2))
        (:`NewEnumerator1`
          (goto _label_3))
        (:`NewEnumerator2`
          (goto _label_3))
        (:`NewEnumerator4`
          (`self.SHOW TEXT` _textrender (`self.Steam Vr Right grip to Grab`)))))
    (:`PSVR`
      (goto _label))))

(event `self.ReceiveBeginPlay`
  (set `self.Scale_0` (`SceneComponent.K2_GetComponentScale` (`self.StaticMeshComponent`)))
  (set `self.Frozen` false))

(event `/Game/Blueprints/Player/LaserState.ToggleState`
  (params (`On/Off` :type Boolean))
  (set `self.Frozen` `On/Off`))

(event `/Game/Blueprints/Player/PickupActorInterface.Pickup`
  (params (AttachTo :type "SceneComponent Object Reference"))
  (`PrimitiveComponent.SetSimulatePhysics` (`self.StaticMeshComponent`) false)
  (`SceneComponent.K2_AttachToComponent` (`self.K2_GetRootComponent`) AttachTo "None" "KeepWorld" "KeepWorld" "KeepWorld" false))

(event `/Game/Blueprints/Player/PickupActorInterface.Drop`
  (`PrimitiveComponent.SetSimulatePhysics` (`self.StaticMeshComponent`) true)
  (`self.K2_DetachFromActor` "KeepWorld" "KeepWorld" "KeepWorld"))

(fn `UserConstructionScript`)