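; Dispenser actor that spawns a configurable class at its Scene component, up to a set total count.
; Tick uses SpawnWithoutActivation, set by ToggleState, as both on/off switch and re-entry gate around the delays.
; Each cycle jumps the dispenser mesh by an offset, spawns after a short delay, then restores the mesh.
; After the spawn interval it re-arms the flag, overriding any mid-cycle switch-off, and increments the count.
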(event `/Game/Blueprints/LaserState.ToggleState`
  (params (`On/Off` :type Boolean))
  (set `self.SpawnWithoutActivation` `On/Off`))

(event `self.ReceiveTick`
  (params (DeltaSeconds :type "Float (single-precision)"))
  (bind _sm_propdespensor_propdis_low (`self.SM_PropDespensor_PropDis_low`))
  (bind _scene (`self.Scene`))
  (bind _returnvalue (`SceneComponent.K2_GetComponentLocation` _sm_propdespensor_propdis_low))
  (bind (_returnvalue_x _returnvalue_y _returnvalue_z) (`KismetMathLibrary.BreakVector` (`SceneComponent.K2_GetComponentLocation` _sm_propdespensor_propdis_low)))
  (if (< (`self.CountObjects`) (`self.HowManyObjects?`))
    (if (`self.SpawnWithoutActivation`)
      (set `self.SpawnWithoutActivation` false)
      (set `self.Inicial Location` _returnvalue)
      (`SceneComponent.K2_SetWorldLocation` (`self.SM_PropDespensor_PropDis_low`) (`KismetMathLibrary.VLerp` _returnvalue (`KismetMathLibrary.MakeVector` (+ _returnvalue_x (`self.Move in X`)) (+ _returnvalue_y (`self.Move in Y`)) (+ _returnvalue_z (`self.Move in Z`))) 1.0) false false)
      (`KismetSystemLibrary.Delay` 0.4)
      (`|SpawnActorFromClass` (`self.ObjectToSpawn`) (`KismetMathLibrary.MakeTransform` (`SceneComponent.K2_GetComponentLocation` _scene) (`SceneComponent.K2_GetComponentRotation` _scene) (`self.Scale Size`)) "AlwaysSpawn" "OverrideRootScale" null null)
      (`SceneComponent.K2_SetWorldLocation` (`self.SM_PropDespensor_PropDis_low`) (`self.Inicial Location`) false false)
      (`KismetSystemLibrary.Delay` (`self.SpawnSeconds`))
      (set `self.SpawnWithoutActivation` true)
      (set `self.CountObjects` (+ (`self.CountObjects`) 1)))))

(fn `UserConstructionScript`)