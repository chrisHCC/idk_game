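; Dispenser actor that spawns a configurable object class, up to a set total, while toggled on and its spawner area holds no pickup cube.
; Tick checks these conditions and fires a DoOnce-gated platform cycle.
; One timeline lerps the platform mesh to a Z offset and spawns the object; a second returns it, resets the gate and increments the count.
; BoxinSpawner overlaps with BP_PickupCube set the blocking flag.
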(event `/Game/Blueprints/Player/LaserState.ToggleState`
  (params (`On/Off` :type Boolean))
  (set `self.SpawnWithoutActivation` `On/Off`))

(event `self.ReceiveBeginPlay`
  (bind (_relativelocation_x _relativelocation_y _relativelocation_z) (`KismetMathLibrary.BreakVector` (`SceneComponent.RelativeLocation` (`self.SM_PropDespensor_PropDis_low`))))
  (set `self.origin` (`SceneComponent.RelativeLocation` (`self.SM_PropDespensor_PropDis_low`)))
  (set `self.target` (`KismetMathLibrary.MakeVector` _relativelocation_x _relativelocation_y (+ _relativelocation_z (`self.z`)))))

(event `self.ReceiveTick`
  (params (DeltaSeconds :type "Float (single-precision)"))
  (if (< (`self.CountObjects`) (`self.HowManyObjects?`))
    (if (`self.IsBox?`)
      _
      (elif (`self.SpawnWithoutActivation`)
        (`/Engine/EditorBlueprintResources/StandardMacros.DoOnce` false :!label _label
          (:`Completed`
            (`self.UP_DoWn_Platform`)))))))

(event `Reset`
  (goto _label :!via `Reset`))

(event `UP_DoWn_Platform`
  (bind (_direction _newtrack_0) (`Timeline|Timeline_0` :!via `PlayFromStart`)
    (:`Update`
      (`SceneComponent.K2_SetRelativeLocation` (`self.SM_PropDespensor_PropDis_low`) (`KismetMathLibrary.VLerp` (`self.origin`) (`self.target`) _newtrack_0) false false))
    (:`Finished`
      (`self.Spawn Object`)
      (bind (_direction_2 _newtrack_0_2) (`Timeline|Timeline_1` :!via `PlayFromStart`)
        (:`Update`
          (`SceneComponent.K2_SetRelativeLocation` (`self.SM_PropDespensor_PropDis_low`) (`KismetMathLibrary.VLerp` (`self.target`) (`self.origin`) _newtrack_0_2) false false))
        (:`Finished`
          (`self.Reset`)
          (set `self.CountObjects` (+ (`self.CountObjects`) 1)))))))

(event `Spawn Object`
  (`|SpawnActorFromClass` (`self.Object to Spawn`) (`KismetMathLibrary.MakeTransform` (`SceneComponent.K2_GetComponentLocation` (`self.spawnpoint`)) (struct) (`self.Scale Object`)) "AdjustIfPossibleButAlwaysSpawn" "OverrideRootScale" null null))

(event `self.BoxinSpawner.OnComponentBeginOverlap`
  (params (OverlappedComponent :type "PrimitiveComponent Object Reference") (OtherActor :type "Actor Object Reference") (OtherComp :type "PrimitiveComponent Object Reference") (OtherBodyIndex :type Integer) (bFromSweep :type Boolean) (SweepResult :type "HitResult Structure (by ref)"))
  (cast `/Game/Blueprints/Player/BP_PickupCube` OtherActor)
  (set `self.IsBox?` true))

(event `self.BoxinSpawner.OnComponentEndOverlap`
  (params (OverlappedComponent :type "PrimitiveComponent Object Reference") (OtherActor :type "Actor Object Reference") (OtherComp :type "PrimitiveComponent Object Reference") (OtherBodyIndex :type Integer))
  (cast `/Game/Blueprints/Player/BP_PickupCube` OtherActor)
  (set `self.IsBox?` false))

(fn `UserConstructionScript`)