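; Dispenser that spawns one configurable object each time it is toggled, ignoring further toggles until its cycle ends.
; A timeline moves the dispenser mesh along its relative Z axis by an offset, then the object spawns at the spawn point with a set scale.
; A second timeline returns the mesh to its origin and resets the DoOnce gate.
; Spawned laser refractors also receive the dispenser's LaserStaysOn setting.
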(event `self.ReceiveBeginPlay`
  (bind (_relativelocation_x _relativelocation_y _relativelocation_z) (`KismetMathLibrary.BreakVector` (`SceneComponent.RelativeLocation` (`self.SM_PropDespensor_PropDis_low`))))
  (set `self.origin` (`SceneComponent.RelativeLocation` (`self.SM_PropDespensor_PropDis_low`)))
  (set `self.target` (`KismetMathLibrary.MakeVector` _relativelocation_x _relativelocation_y (+ _relativelocation_z (`self.z`)))))

(event `/Game/Blueprints/Player/LaserState.ToggleState`
  (params (`On/Off` :type Boolean))
  (`/Engine/EditorBlueprintResources/StandardMacros.DoOnce` false :!label _label
    (:`Completed`
      (`self.UP_DoWn_Platform`))))

(event `Reset`
  (goto _label :!via `Reset`))

(event `UP_DoWn_Platform`
  (bind (_direction _newtrack_0) (`Timeline|Timeline_0` :!via `PlayFromStart`)
    (:`Update`
      (`SceneComponent.K2_SetRelativeLocation` (`self.SM_PropDespensor_PropDis_low`) (`KismetMathLibrary.VLerp` (`self.origin`) (`self.target`) _newtrack_0) false false))
    (:`Finished`
      (`self.Spawn Object`)
      (bind (_direction_2 _newtrack_0_2) (`Timeline|Timeline_1` :!via `PlayFromStart`)
        (:`Update`
          (`SceneComponent.K2_SetRelativeLocation` (`self.SM_PropDespensor_PropDis_low`) (`KismetMathLibrary.VLerp` (`self.target`) (`self.origin`) _newtrack_0_2) false false))
        (:`Finished`
          (`self.Reset`))))))

(event `Spawn Object`
  (bind _returnvalue (`|SpawnActorFromClass` (`self.Object to Spawn`) (`KismetMathLibrary.MakeTransform` (`SceneComponent.K2_GetComponentLocation` (`self.spawnpoint`)) (struct) (`self.Scale Object`)) "AdjustIfPossibleButAlwaysSpawn" "OverrideRootScale" null null))
  (if (== (`self.Object to Spawn`) "/Game/Blueprints/laser_refractor/BP_LaserRefractor.BP_LaserRefractor_C")
    (bind _asbp_laser_refractor (cast `/Game/Blueprints/laser_refractor/BP_LaserRefractor` _returnvalue))
    (set `/Game/Blueprints/laser_refractor/BP_LaserRefractor.laser stays on` (`self.Laser stays on`) _asbp_laser_refractor)))

(fn `UserConstructionScript`)