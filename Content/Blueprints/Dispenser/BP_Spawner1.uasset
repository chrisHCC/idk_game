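; BP_Spawner1 is a dispenser Blueprint that spawns a configurable class at its Scene component's transform, up to a set object count.
; Tick starts each cycle while SpawnWithoutActivation is true, clearing that flag during a short pre-spawn delay and SpawnSeconds cooldown, then restoring it and incrementing the count.
; ToggleState writes the same flag, so switching off mid-cycle is overridden when the cooldown ends.
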(event `/Game/Blueprints/LaserState.ToggleState`
  (params (`On/Off` :type Boolean))
  (set `self.SpawnWithoutActivation` `On/Off`))

(event `self.ReceiveTick`
  (params (DeltaSeconds :type "Float (single-precision)"))
  (bind _scene (`self.Scene`))
  (if (< (`self.CountObjects`) (`self.HowManyObjects?`))
    (if (`self.SpawnWithoutActivation`)
      (set `self.SpawnWithoutActivation` false)
      (`KismetSystemLibrary.Delay` 0.4)
      (`|SpawnActorFromClass` (`self.ObjectToSpawn`) (`KismetMathLibrary.MakeTransform` (`SceneComponent.K2_GetComponentLocation` _scene) (`SceneComponent.K2_GetComponentRotation` _scene) (`self.Scale Size`)) "AlwaysSpawn" "OverrideRootScale" null null)
      (`KismetSystemLibrary.Delay` (`self.SpawnSeconds`))
      (set `self.SpawnWithoutActivation` true)
      (set `self.CountObjects` (+ (`self.CountObjects`) 1)))))

(fn `UserConstructionScript`)